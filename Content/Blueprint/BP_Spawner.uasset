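; BP_Spawner spawns a random mask pickup at its SpawnPoint on BeginPlay and respawns another after it is picked up.
; SpawnRandom creates a BP_MaskParent, initializes it with a random row name from MaskTable, and returns it.
; Respawn binds the mask's OnPickup, which starts a SpawnTime timer back to Respawn.
; The debug print re-rolls the random index, so its logged name can differ from the spawned mask.
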(event Custom|Respawn
  (bind _newparam (CallFunction|SpawnRandom))
  (EventDispatchers|BindEventtoOnPickup _newparam (delegate Custom|OnPickup)))

(event Custom|OnPickup
  (Utilities|Time|SetTimerbyEvent (delegate Custom|Respawn) (Variables|Default|GetSpawnTime)))

(event EventBeginPlay
  (CallFunction|Respawn))

(event Collision|EventActorBeginOverlap
  (params (OtherActor :type Actor%20Object%20Reference)))

(fn ConstructionScript)

(fn SpawnRandom
  (bind _outrownames (DataTable|GetDataTableRowNames (Variables|Default|GetMaskTable)))
  (bind _returnvalue (Game|SpawnActorfromClass "/Game/Blueprint/Masks/BP_MaskParent.BP_MaskParent_C" (Transformation|GetWorldTransform (Variables|Default|GetSpawnPoint)) "Undefined" "MultiplyWithRoot" 0 0))
  (Default|Initialize _returnvalue (Utilities|Array|Get(acopy) _outrownames (Math|Random|RandomInteger (Utilities|Array|Length _outrownames))))
  (Development|PrintString (Utilities|String|Append "Spawned " (Utilities|String|ToString(Name) (Utilities|Array|Get(acopy) _outrownames (Math|Random|RandomInteger (Utilities|Array|Length _outrownames))))))
  (return _returnvalue))