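; BP_Camera is a shared orthographic camera for two players that switches to split screen when they move apart.
; Each Tick it places its Billboard at the midpoint between both players and sets ortho width from their clamped distance.
; A looping one-second timer checks that distance, disabling split screen and viewing this camera when close, otherwise enabling it and pointing the first controller at PlayerOne.
; Both player references are supplied through setter events.
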(event Custom|Set%20Player%20Ref
  (params (Player%20One%20Ref :type BP%20Player%20One%20Object%20Reference))
  (Variables|PlayerRef|SetPlayer%20One Player%20One%20Ref))

(event Custom|Set%20Player%20Tow%20Ref
  (params (Player%20Tow%20Ref :type BP%20Player%20Two%20Object%20Reference))
  (Variables|PlayerRef|SetPlayer%20Tow Player%20Tow%20Ref))

(event Custom|Check%20Player%20Distance%20For%20Spli%20Cam
  (bind _player_one (Variables|PlayerRef|GetPlayer%20One))
  (bind _player_tow (Variables|PlayerRef|GetPlayer%20Tow))
  (bind _returnvalue (Transformation|GetDistanceTo _player_one _player_tow))
  (bind _returnvalue_2 (<= _returnvalue 1.5e+03))
  ;[0.15 0.15 0.15 0.5] Switch
  (Class|GameplayStatics|SetForceDisableSplitscreen _returnvalue_2)
  (if _returnvalue_2
    (Game|Player|SetViewTargetwithBlend (Game|GetPlayerController 0) self 0.0 "VTBlend_Linear" 0.0 false)
    (else
      (Game|Player|SetViewTargetwithBlend (Game|GetPlayerController 0) (Variables|PlayerRef|GetPlayer%20One) 0.0 "VTBlend_Linear" 0.0 false))))

(event EventBeginPlay
  (Class|GameplayStatics|SetForceDisableSplitscreen true)
  (Game|Player|SetViewTargetwithBlend (Game|GetPlayerController 0) self 0.0 "VTBlend_Linear" 0.0 false)
  (Utilities|Time|SetTimerbyFunctionName 0 "Check Player Distance For Spli Cam" 1.0 true))

(event EventTick
  (params (DeltaSeconds :type Float%20%28single-precision%29))
  (Class|CameraComponent|SetOrthoWidth (Variables|Default|GetCamera) (Math|Float|Clamp(Float) (Transformation|GetDistanceTo (Variables|PlayerRef|GetPlayer%20One) (Variables|PlayerRef|GetPlayer%20Tow)) 768.0 1.5e+03))
  (bind _output_get (Variables|Default|SetCamera%20Location (Math|Vector|Lerp(Vector) (Transformation|GetActorLocation (Variables|PlayerRef|GetPlayer%20One)) (Transformation|GetActorLocation (Variables|PlayerRef|GetPlayer%20Tow)) 0.5)))
  (Transformation|SetWorldLocation (Variables|Default|GetBillboard) _output_get false false))

(fn ConstructionScript)