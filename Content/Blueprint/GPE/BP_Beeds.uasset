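; BP_Beeds is a boid actor that flocks with other BP_Beeds while avoiding walls.
; A looping timer scans all instances, blending nested-radius cohesion, alignment and separation plus planar random jitter into Direction, with debug circles.
; Tick moves the actor along Direction at Speed, facing it.
; Each tick, two angled line traces detect obstacles and rotate Direction around Z, turning the same way whichever side is closer.
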(event Custom|Update
  (bind _returnvalue (Math|Random|RandomUnitVector))
  (Variables|Default|SetCohesionDir "0, 0, 0")
  (Variables|Default|SetAlignmentDir "0, 0, 0")
  (Variables|Default|SetSeparationDir "0, 0, 0")
  (Variables|Default|SetCohesionCount 0)
  (Variables|Default|SetAlignmentCount 0)
  (Variables|Default|SetSeparationCount 0)
  (bind _outactors (Actor|GetAllActorsOfClass "BP_Beeds_C"))
  (for _array_element _outactors
    (if (not (== _array_element self))
      ;[0.15 0.15 0.15 0.5] Cohesion
      (if (< (Math|Vector|VectorLengthSquared (- (Transformation|GetActorLocation _array_element) (Transformation|GetActorLocation))) (Variables|Default|GetCohesion))
        (Variables|Default|SetCohesionDir (+ (Math|Vector|Normalize (- (Transformation|GetActorLocation _array_element) (Transformation|GetActorLocation))) (Variables|Default|GetCohesionDir)))
        (Math|Integer|IncrementInt (Variables|Default|GetCohesionCount)
          (:%20%20
            (Rendering|Debug|DrawDebugCircle (Transformation|GetActorLocation) (Math|Float|Sqrt (Variables|Default|GetCohesion)) 24 "(R=1.000000,G=0.000000,B=0.008407,A=1.000000)" (Variables|Default|GetUpdateRate) 1.0 "1.000000,0.000000,0.000000" "0.000000,1.000000,0.000000")
            ;[0.15 0.15 0.15 0.5] Alignment
            (if (< (Math|Vector|VectorLengthSquared (- (Transformation|GetActorLocation _array_element) (Transformation|GetActorLocation))) (Variables|Default|GetAlignment))
              (Variables|Default|SetAlignmentDir (+ (Variables|Default|GetAlignmentDir) (Transformation|GetActorForwardVector _array_element)))
              (Math|Integer|IncrementInt (Variables|Default|GetAlignmentCount)
                (:%20%20
                  (Rendering|Debug|DrawDebugCircle (Transformation|GetActorLocation) (Math|Float|Sqrt (Variables|Default|GetAlignment)) 24 "(R=0.166425,G=1.000000,B=0.000000,A=1.000000)" (Variables|Default|GetUpdateRate) 1.0 "1.000000,0.000000,0.000000" "0.000000,1.000000,0.000000")
                  ;[0.15 0.15 0.15 0.5] Cohesion
                  (if (< (Math|Vector|VectorLengthSquared (- (Transformation|GetActorLocation _array_element) (Transformation|GetActorLocation))) (Variables|Default|GetSeparation))
                    (Variables|Default|SetSeparationDir (- (Variables|Default|GetSeparationDir) (Math|Vector|Normalize (- (Transformation|GetActorLocation _array_element) (Transformation|GetActorLocation)))))
                    (Math|Integer|IncrementInt (Variables|Default|GetSeparationCount)
                      (:%20%20
                        (Rendering|Debug|DrawDebugCircle (Transformation|GetActorLocation) (Math|Float|Sqrt (Variables|Default|GetSeparation)) 12 "(R=0.000000,G=0.069023,B=1.000000,A=1.000000)" (Variables|Default|GetUpdateRate) 1.0 "1.000000,0.000000,0.000000" "0.000000,1.000000,0.000000"))))))))))))
  ;[0.15 0.15 0.15 0.5] Combine
  (Variables|Default|SetDirection (Math|Vector|Normalize (Math|Vector|Lerp(Vector) (Variables|Default|GetDirection) (Math|Vector|Normalize (+ (* (Math|Vector|MakeVector (.x _returnvalue) (.y _returnvalue) 0.0) (Variables|Default|GetRandomStrength)) (+ (+ (* (/ (Variables|Default|GetCohesionDir) (Variables|Default|GetCohesionCount)) (Variables|Default|GetCohesionStrength)) (* (/ (Variables|Default|GetAlignmentDir) (Variables|Default|GetAlignmentCount)) (Variables|Default|GetAlignmentStrength))) (* (/ (Variables|Default|GetSeparationDir) (Variables|Default|GetSeparationCount)) (Variables|Default|GetSeparationStrength))))) (* (Variables|Default|GetRotateSpeed) (Variables|Default|GetUpdateRate))))))

(event EventBeginPlay
  (Utilities|Time|SetTimerbyEvent (delegate Custom|Update) (Variables|Default|GetUpdateRate) true true))

(event EventTick
  (params (DeltaSeconds :type Float%20%28single-precision%29))
  (bind _direction (Variables|Default|GetDirection))
  (CallFunction|AvoidWalls)
  (Transformation|SetActorLocationAndRotation (+ (* DeltaSeconds (* _direction (Variables|Default|GetSpeed))) (Transformation|GetActorLocation)) (Math|Rotator|CombineRotators (Math|Rotator|MakeRotfromX _direction) "0.000000,-90.000000,0.000000")))

(fn ConstructionScript)

(fn AvoidWalls
  (bind _returnvalue (Transformation|GetActorLocation))
  (bind _returnvalue_2 (Transformation|GetActorLocation))
  (bind _outhit (Collision|LineTraceByChannel _returnvalue_2 (+ _returnvalue_2 (* (Math|Vector|RotateVectorAroundAxis (Variables|Default|GetDirection) -15.0 "0.000000,0.000000,1.000000") (LocalVariables|GetDistance))) "TraceTypeQuery1" false 0 "ForOneFrame"))
  (bind _outhit_2 (Collision|LineTraceByChannel _returnvalue (+ _returnvalue (* (Math|Vector|RotateVectorAroundAxis (Variables|Default|GetDirection) 15.0 "0.000000,0.000000,1.000000") (LocalVariables|GetDistance))) "TraceTypeQuery1" false 0 "ForOneFrame"))
  (if (or (.bblockinghit _outhit) (.bblockinghit _outhit_2))
    (if (< (.distance _outhit) (.distance _outhit_2))
      (Variables|Default|SetDirection (Math|Vector|RotateVectorAroundAxis (Variables|Default|GetDirection) (Variables|Default|GetAvoidWallStrength) "0.000000,0.000000,1.000000"))
      (else
        (Variables|Default|SetDirection (Math|Vector|RotateVectorAroundAxis (Variables|Default|GetDirection) (Variables|Default|GetAvoidWallStrength) "0.000000,0.000000,1.000000"))))))