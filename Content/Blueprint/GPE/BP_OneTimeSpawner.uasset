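; One-time spawner GPE that places a single mask pickup in the level and destroys itself once that mask is picked up.
; On BeginPlay it spawns a BP_MaskParent at SpawnPoint, initializes it with the Mask row name and binds to its pickup event.
; The MaskTable row's type selects the Distance, Melee or Support hollow Niagara effect, which is deactivated on pickup before the spawner is destroyed.
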(event Custom|OnMaskPickup
  (Components|Activation|Deactivate (Variables|Default|GetNS_MaskHollowPickup))
  (Actor|DestroyActor))

(event EventBeginPlay
  (bind _newparam (CallFunction|SpawnMask))
  (EventDispatchers|BindEventtoOnPickup _newparam (delegate Custom|OnMaskPickup)))

(event Collision|EventActorBeginOverlap
  (params (OtherActor :type Actor%20Object%20Reference)))

(fn ConstructionScript)

(fn SpawnMask
  (bind _mask (Variables|Default|GetMask))
  (bind _ns_maskhollowpickup (Variables|Default|GetNS_MaskHollowPickup))
  (bind _returnvalue (Game|SpawnActorfromClass "/Game/Blueprint/Masks/BP_MaskParent.BP_MaskParent_C" (Transformation|GetWorldTransform (Variables|Default|GetSpawnPoint)) "Undefined" "MultiplyWithRoot" 0 0))
  (Default|Initialize _returnvalue _mask)
  (Development|PrintString (Utilities|String|Append "Spawned " (Utilities|String|ToString(Name) _mask)))
  (bind _returnvalue_2 (Utilities|GetDataTableRow (Variables|Default|GetMaskTable) _mask)
    (:then
      (Components|Activation|Activate (Variables|Default|GetNS_MaskHollowPickup) false)
      (switch Utilities|FlowControl|Switch|SwitchonENUM_MaskType (.Type (Utilities|Struct|BreakS_MaskList _returnvalue_2))
        (:NewEnumerator0
          (Class|NiagaraComponent|SetAsset _ns_maskhollowpickup "/Game/VFX/Halo/NS_MaskHollowDistance.NS_MaskHollowDistance" true))
        (:NewEnumerator1
          (Class|NiagaraComponent|SetAsset _ns_maskhollowpickup "/Game/VFX/Halo/NS_MaskHollowMelee.NS_MaskHollowMelee" true))
        (:NewEnumerator2
          (Class|NiagaraComponent|SetAsset _ns_maskhollowpickup "/Game/VFX/Halo/NS_MaskHollowSupport.NS_MaskHollowSupport" true))))
    (:RowNotFound
      _))
  (return _returnvalue _mask))