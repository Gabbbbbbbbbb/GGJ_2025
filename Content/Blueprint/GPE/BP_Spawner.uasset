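; Mask pickup spawner that spawns a random mask at its spawn point on BeginPlay and again after each pickup.
; SpawnRandom initializes a BP_MaskParent from a MaskTable row and sets a Niagara effect by mask type (distance, melee, support).
; Pickup deactivates the effect and runs a timeline that drives the WBP_Timer slider until respawn.
; The random row is re-rolled per use, so effect and mask can differ.
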(event Custom|OnPickup
  (Components|Activation|Deactivate (Variables|Default|GetNS_MaskHollowPickup))
  (bind _countdown (Timeline|Timeline Play)
    (:Update
      (bind _aswbp_timer (Utilities|Casting|CastToWBP_Timer (UserInterface|GetWidget (Variables|Default|GetWidget))))
      (Class|RadialSlider|SetValue (Variables|/Game/Blueprint/GPE/WBP_Timer.WBP_Timer_C|GetSlider _aswbp_timer) _countdown))
    (:Finished
      (bind _newparam (CallFunction|SpawnRandom))
      (EventDispatchers|BindEventtoOnPickup _newparam (delegate Custom|OnPickup)))))

(event EventBeginPlay
  (bind _newparam (CallFunction|SpawnRandom))
  (EventDispatchers|BindEventtoOnPickup _newparam (delegate Custom|OnPickup))
  (bind _aswbp_timer (Utilities|Casting|CastToWBP_Timer (UserInterface|GetWidget (Variables|Default|GetWidget))))
  (Class|RadialSlider|SetValue (Variables|/Game/Blueprint/GPE/WBP_Timer.WBP_Timer_C|GetSlider _aswbp_timer) 0.0))

(event Collision|EventActorBeginOverlap
  (params (OtherActor :type Actor%20Object%20Reference)))

(fn ConstructionScript)

(fn SpawnRandom
  (bind _ns_maskhollowpickup (Variables|Default|GetNS_MaskHollowPickup))
  (bind _outrownames (DataTable|GetDataTableRowNames (Variables|Default|GetMaskTable)))
  (bind _returnvalue (Game|SpawnActorfromClass "/Game/Blueprint/Masks/BP_MaskParent.BP_MaskParent_C" (Transformation|GetWorldTransform (Variables|Default|GetSpawnPoint)) "Undefined" "MultiplyWithRoot" 0 0))
  (Default|Initialize _returnvalue (Utilities|Array|Get(acopy) _outrownames (Math|Random|RandomInteger (Utilities|Array|Length _outrownames))))
  (bind _returnvalue_2 (Utilities|GetDataTableRow (Variables|Default|GetMaskTable) (Utilities|Array|Get(acopy) _outrownames (Math|Random|RandomInteger (Utilities|Array|Length _outrownames))))
    (:then
      (Components|Activation|Activate (Variables|Default|GetNS_MaskHollowPickup) false)
      (switch Utilities|FlowControl|Switch|SwitchonENUM_MaskType (.Type (Utilities|Struct|BreakS_MaskList _returnvalue_2))
        (:NewEnumerator0
          (Class|NiagaraComponent|SetAsset _ns_maskhollowpickup "/Game/VFX/Halo/NS_MaskHollowPickupDistance.NS_MaskHollowPickupDistance" true))
        (:NewEnumerator1
          (Class|NiagaraComponent|SetAsset _ns_maskhollowpickup "/Game/VFX/Halo/NS_MaskHollowPickupMelee.NS_MaskHollowPickupMelee" true))
        (:NewEnumerator2
          (Class|NiagaraComponent|SetAsset _ns_maskhollowpickup "/Game/VFX/Halo/NS_MaskHollowPickupSupport.NS_MaskHollowPickupSupport" true))))
    (:RowNotFound
      _))
  (return _returnvalue (Utilities|Array|Get(acopy) _outrownames (Math|Random|RandomInteger (Utilities|Array|Length _outrownames)))))