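; Actor component that manages the masks a player collects.
; On PickUp it stores the mask's class in a distance, melee or support array according to its MaskType.
; It then calls AddMaskMesh, which casts the picking actor to BP_PlayerParent to add the mask's static mesh, printing a debug message if the cast fails.
; The Hit function is an empty stub.
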(event EventBeginPlay)

(event EventTick
  (params (DeltaSeconds :type Float%20%28single-precision%29)))

(event EventPickUp
  (params (PickedMask :type BP%20Mask%20Parent%20Object%20Reference) (Actor :type Actor%20Object%20Reference))
  (Variables|Default|SetActor Actor)
  (bind _output_get (Variables|Default|SetPicked%20Mask PickedMask))
  (switch Utilities|FlowControl|Switch|SwitchonENUM_MaskType (Variables|/Game/Blueprint/Masks/BP_MaskParent.BP_MaskParent_C|GetMaskType _output_get)
    (:NewEnumerator0
      (Utilities|Array|Add (Variables|Default|GetDistanceMasks) (Utilities|GetClass PickedMask)))
    (:NewEnumerator1
      (Utilities|Array|Add (Variables|Default|GetMeleeMasks) (Utilities|GetClass PickedMask)))
    (:NewEnumerator2
      (Utilities|Array|Add (Variables|Default|GetSupportMasks) (Utilities|GetClass PickedMask))))
  (CallFunction|AddMaskMesh))

(fn AddMaskMesh
  (bind _asbp_player_parent (Utilities|Casting|CastToBP_PlayerParent (Variables|Default|GetActor))
    (:then
      (Default|AddStaticMesh _asbp_player_parent (Variables|Default|GetPicked%20Mask)))
    (:CastFailed
      (Development|PrintString "AddMaskMesh cast failed" true true "(R=0.925294,G=1.000000,B=0.842948,A=1.000000)" 5.0 "1"))))

(fn Hit)