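; Base actor for mask pickups that a player collects by touching them.
; Initialize looks up a row in MaskTable by mask name, sets the static mesh from it and stores the name.
; When the sphere overlaps a BP_PlayerParent, it passes the mask name to that player's AC_MaskManager through PickUpMessage, then destroys itself.
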(event OnComponentBeginOverlap(Sphere)
  (params (OverlappedComponent :type Primitive%20Component%20Object%20Reference) (OtherActor :type Actor%20Object%20Reference) (OtherComp :type Primitive%20Component%20Object%20Reference) (OtherBodyIndex :type Integer) (bFromSweep :type Boolean) (SweepResult :type Hit%20Result%20Structure%20%28by%20ref%29))
  (Class|KismetSystemLibrary|IsObjectOfSoftClass OtherActor "/Game/Blueprint/Players/BP_PlayerParent.BP_PlayerParent_C"
    (:True
      (Class|BPIInteract|PickUp(Message) (Actor|GetComponentbyClass OtherActor "/Game/Blueprint/Masks/AC_MaskManager.AC_MaskManager_C") (Variables|Default|GetMask%20Name) OtherActor)
      (Actor|DestroyActor))))

(fn ConstructionScript)

(fn Initialize
  (params (MaskName :type Name))
  (bind _returnvalue (Utilities|GetDataTableRow (Variables|Default|GetMaskTable) MaskName)
    (:then
      (Components|StaticMesh|SetStaticMesh (Variables|Default|GetMesh) (.Mesh (Utilities|Struct|BreakS_MaskList _returnvalue)))
      (Variables|Default|SetMask%20Name MaskName))))