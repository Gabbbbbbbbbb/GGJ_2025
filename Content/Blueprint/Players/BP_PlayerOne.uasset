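; BP_PlayerOne is a player Blueprint, by its name the first player, that adds camera registration and input setup on top of its parent class.
; On BeginPlay it runs the parent logic, then finds the BP_Camera actor in the level and passes itself as the player reference.
; It then casts its controller to PlayerController and adds the IMC_Players mapping context to the Enhanced Input subsystem.
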(event EventBeginPlay
  (|CallParentFunction)
  (bind _returnvalue (Actor|GetActorOfClass "/Game/Blueprint/Camera/BP_Camera.BP_Camera_C"))
  (Default|SetPlayerRef _returnvalue self)
  (bind _asplayer_controller (Utilities|Casting|CastToPlayerController (Pawn|GetController)))
  (Utilities|IsValid (PlayerController|LocalPlayerSubsystems|GetEnhancedInputLocalPlayerSubsystem _asplayer_controller)
    (:Is%20Valid
      (Input|AddMappingContext (PlayerController|LocalPlayerSubsystems|GetEnhancedInputLocalPlayerSubsystem _asplayer_controller) "/Game/Blueprint/Players/Inputs/IMC_Players.IMC_Players" 0 "(bIgnoreAllPressedKeysUntilRelease=True,bForceImmediately=False,bNotifyUserSettings=False)"))))

(fn ConstructionScript
  (|CallParentFunction))