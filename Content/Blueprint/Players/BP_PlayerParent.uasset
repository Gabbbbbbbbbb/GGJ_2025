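; Parent player Character that moves relative to the camera, dashes along its velocity with a cooldown, and scales its sphere mesh with speed.
; Distance, Support and Melee inputs spawn every actor class in the matching ACMaskManager mask list at front or ground reference points.
; AddStaticMesh chains collision-free mask meshes, each offset from the last, and records them in the manager.
; Pause input shows HUD_Main's pause menu, stops the in-game timer and pauses the game.
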(event Input|EnhancedActionEvents|EnhancedInputActionIA_Move
  (params (ActionValue :type Vector%202D%20Structure) (ElapsedSeconds :type Float%20%28double-precision%29) (TriggeredSeconds :type Float%20%28double-precision%29) (InputAction :type Input%20Action%20Object%20Reference :default "/Game/Blueprint/Players/Inputs/Actions/IA_Move.IA_Move"))
  (bind _returnvalue (Game|GetPlayerCameraManager 0))
  (bind _transformcomponent (Variables|/Script/Engine.PlayerCameraManager|GetTransformComponent _returnvalue))
  ;[0.15 0.15 0.15 0.5] Move Set
  (Pawn|Input|AddMovementInput (Math|Vector|GetForwardVector _transformcomponent) (.y ActionValue) false)
  (Pawn|Input|AddMovementInput (Math|Vector|GetRightVector _transformcomponent) (.x ActionValue) false))

(event Input|EnhancedActionEvents|EnhancedInputActionIA_Distance
  (params (ActionValue :type Boolean) (ElapsedSeconds :type Float%20%28double-precision%29) (TriggeredSeconds :type Float%20%28double-precision%29) (InputAction :type Input%20Action%20Object%20Reference :default "/Game/Blueprint/Players/Inputs/Actions/IA_Distance.IA_Distance"))
  (for _array_element (Variables|/Game/Blueprint/Masks/AC_MaskManager.AC_MaskManager_C|GetDistanceMasks (Variables|Default|GetAC_MaskManager))
    (Game|SpawnActorfromClass _array_element (Transformation|GetWorldTransform (Variables|Default|GetFrontReference)) "Undefined" "MultiplyWithRoot" 0 (Variables|Default|GetID) 0)))

(event Input|EnhancedActionEvents|EnhancedInputActionIA_Melee
  (params (ActionValue :type Boolean) (ElapsedSeconds :type Float%20%28double-precision%29) (TriggeredSeconds :type Float%20%28double-precision%29) (InputAction :type Input%20Action%20Object%20Reference :default "/Game/Blueprint/Players/Inputs/Actions/IA_Melee.IA_Melee"))
  (for _array_element (Variables|/Game/Blueprint/Masks/AC_MaskManager.AC_MaskManager_C|GetMeleeMasks (Variables|Default|GetAC_MaskManager))
    (Game|SpawnActorfromClass _array_element (Transformation|GetWorldTransform (Variables|Default|GetFrontReference)) "Undefined" "MultiplyWithRoot" 0 (Variables|Default|GetID) 0)))

(event Input|EnhancedActionEvents|EnhancedInputActionIA_Support
  (params (ActionValue :type Boolean) (ElapsedSeconds :type Float%20%28double-precision%29) (TriggeredSeconds :type Float%20%28double-precision%29) (InputAction :type Input%20Action%20Object%20Reference :default "/Game/Blueprint/Players/Inputs/Actions/IA_Support.IA_Support"))
  (for _array_element (Variables|/Game/Blueprint/Masks/AC_MaskManager.AC_MaskManager_C|GetSupportMasks (Variables|Default|GetAC_MaskManager))
    (Game|SpawnActorfromClass _array_element (Transformation|GetWorldTransform (Variables|Default|GetGroundRefernce)) "Undefined" "MultiplyWithRoot" 0 (Variables|Default|GetID) 0)))

(event Input|EnhancedActionEvents|EnhancedInputActionIA_Pause
  (params (ActionValue :type Boolean) (ElapsedSeconds :type Float%20%28double-precision%29) (TriggeredSeconds :type Float%20%28double-precision%29) (InputAction :type Input%20Action%20Object%20Reference :default "/Game/Blueprint/Players/Inputs/Actions/IA_Pause.IA_Pause"))
  (bind _refhudmain (Variables|Default|GetRefHUDMain)
    (:then
      (Default|ResetVisibility (Variables|/Game/_GameManager/HUD_Main.HUD_Main_C|GetRefPauseMenu _refhudmain))
      (Widget|SetVisibility (Variables|/Game/_GameManager/HUD_Main.HUD_Main_C|GetRefPauseMenu _refhudmain) "Visible")
      (Variables|/Game/UI/InGameMenu/WBP_InGameMenu.WBP_InGameMenu_C|SetbIsTimerRunning (Variables|/Game/_GameManager/HUD_Main.HUD_Main_C|GetRefInGameMenu (Variables|Default|GetRefHUDMain)) false)
      (Game|SetGamePaused true))
    (:else)))

(event Input|EnhancedActionEvents|EnhancedInputActionIA_Dash
  (params (ActionValue :type Boolean) (ElapsedSeconds :type Float%20%28double-precision%29) (TriggeredSeconds :type Float%20%28double-precision%29) (InputAction :type Input%20Action%20Object%20Reference :default "/Game/Blueprint/Players/Inputs/Actions/IA_Dash.IA_Dash"))
  (bind _returnvalue (Transformation|GetVelocity))
  (bind _dash_force (Variables|Dash|GetDash%20Force))
  (bind _returnvalue_2 (* _returnvalue _dash_force))
  ;[0.15 0.15 0.15 0.5] Move Set
  (if (not (Variables|Dash|GetDash))
    (Variables|Dash|SetDash true)
    (Character|LaunchCharacter (Math|Vector|MakeVector (.x _returnvalue_2) (.y _returnvalue_2) 0.0) false false)
    (Utilities|FlowControl|Delay (Variables|Dash|GetDash%20Delay))
    (Variables|Dash|SetDash false)))

(event EventBeginPlay
  (bind _ashud_main (Utilities|Casting|CastToHUD_Main (HUD|GetHUD (Game|GetPlayerController 0))))
  (Variables|Default|SetRefHUDMain _ashud_main)
  (Variables|Default|SetBaseScale (Variables|/Script/Engine.SceneComponent|GetRelativeScale3D (Variables|Default|GetSphere))))

(event EventTick
  (params (DeltaSeconds :type Float%20%28single-precision%29))
  (Transformation|SetRelativeScale3D (Variables|Default|GetSphere) (Math|Vector|Lerp(Vector) (Variables|Default|GetBaseScale) (Variables|Default|GetMaxScale) (/ (Math|Vector|VectorLength (Transformation|GetVelocity)) (Class|MovementComponent|GetMaxSpeed (Variables|Character|GetCharacterMovement))))))

(fn ConstructionScript)

(fn AddStaticMesh
  (params (Mesh :type Static%20Mesh%20Object%20Reference))
  (bind _ac_maskmanager (Variables|Default|GetAC_MaskManager))
  (bind _wornmasks_mesh (Variables|/Game/Blueprint/Masks/AC_MaskManager.AC_MaskManager_C|GetWornMasks_Mesh _ac_maskmanager))
  (if (Utilities|Array|IsEmpty _wornmasks_mesh)
    ;[0.15 0.15 0.15 0.5] If the player isn't wearing any mask
    (bind _returnvalue (AddComponent|AddStaticMeshComponent false (Math|Transform|MakeTransform (+ (Variables|/Script/Engine.SceneComponent|GetRelativeLocation (Variables|Default|GetSphere)) "50.000000,0.000000,0.000000"))))
    (Components|StaticMesh|SetStaticMesh _returnvalue Mesh)
    (Collision|SetCollisionEnabled _returnvalue "NoCollision")
    (Utilities|Array|Add (Variables|/Game/Blueprint/Masks/AC_MaskManager.AC_MaskManager_C|GetWornMasks_Mesh (Variables|Default|GetAC_MaskManager)) _returnvalue)
    (else
      ;[0.15 0.15 0.15 0.5] If the player is already wearing a mask
      (bind _returnvalue_2 (AddComponent|AddStaticMeshComponent false (Math|Transform|MakeTransform (+ (Variables|/Script/Engine.SceneComponent|GetRelativeLocation (Utilities|Array|Get(acopy) _wornmasks_mesh (Utilities|Array|LastIndex _wornmasks_mesh))) "50.000000,0.000000,0.000000"))))
      (Components|StaticMesh|SetStaticMesh _returnvalue_2 Mesh)
      (Collision|SetCollisionEnabled _returnvalue_2 "NoCollision")
      (Utilities|Array|Add (Variables|/Game/Blueprint/Masks/AC_MaskManager.AC_MaskManager_C|GetWornMasks_Mesh (Variables|Default|GetAC_MaskManager)) _returnvalue_2))))