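; Flocking boid projectile with flapping wings that belongs to one of two teams and damages the opposing player on overlap, then destroys itself.
; A looping timer blends same-team cohesion, alignment and separation, randomness, and opposing-player direction within range into a planar heading.
; Tick moves it along that heading after two angled traces check for walls; both hit branches turn it the same way.
; Initialize sets team, heading and mesh.
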(event Custom|Update
  (bind _returnvalue (Transformation|GetActorLocation))
  (bind _team (Variables|Default|GetTeam))
  (bind _boidinfo (Variables|Default|GetBoidInfo))
  (bind _boidinfo_2 (Variables|Default|GetBoidInfo))
  (bind _returnvalue_2 (Math|Conversions|ToBoolean(Integer) _team))
  (bind _returnvalue_3 (!= _returnvalue_2 true))
  (bind _returnvalue_4 (Math|Conversions|ToInteger(Boolean) _returnvalue_3))
  (bind _returnvalue_5 (Class|GameplayStatics|GetPlayerControllerfromID _returnvalue_4))
  (bind _returnvalue_6 (Pawn|GetControlledPawn _returnvalue_5))
  (bind _returnvalue_7 (Transformation|GetActorLocation _returnvalue_6))
  (bind _returnvalue_8 (- _returnvalue_7 _returnvalue))
  (Variables|Default|SetCohesionDir "0, 0, 0")
  (Variables|Default|SetAlignmentDir "0, 0, 0")
  (Variables|Default|SetSeparationDir "0, 0, 0")
  (bind _outactors (Actor|GetAllActorsOfClass "BP_Beeds_C"))
  (for _array_element _outactors
    (if (not (== _array_element self)) ; Ignore self
      (if (== (Variables|BP_Beeds_C|GetTeam _array_element) (Variables|Default|GetTeam)) ; true -> friend algo
        ;[0.05166 0.15 0 0.5] Friend
        ;;[0.15 0.00652 0 0.5] Cohesion
        (if (< (Math|Vector|VectorLengthSquared (- (Transformation|GetActorLocation _array_element) (Transformation|GetActorLocation))) (.cohesionrangesqr _boidinfo))
          (Variables|Default|SetCohesionDir (+ (Math|Vector|Normalize (- (Transformation|GetActorLocation _array_element) (Transformation|GetActorLocation))) (Variables|Default|GetCohesionDir)))
          ;;[0.000828 0.15 0 0.5] Alignment
          (if (< (Math|Vector|VectorLengthSquared (- (Transformation|GetActorLocation _array_element) (Transformation|GetActorLocation))) (.alignmentrangesqr _boidinfo))
            (Variables|Default|SetAlignmentDir (+ (Variables|Default|GetAlignmentDir) (Variables|BP_Beeds_C|GetDirection _array_element)))
            ;;[0 0.001113 0.15 0.5] Separation
            (if (< (Math|Vector|VectorLengthSquared (- (Transformation|GetActorLocation _array_element) (Transformation|GetActorLocation))) (.separationrangesqr _boidinfo))
              (Variables|Default|SetSeparationDir (- (Variables|Default|GetSeparationDir) (Math|Vector|Normalize (- (Transformation|GetActorLocation _array_element) (Transformation|GetActorLocation)))))))))))
  ;[0.15 0.1213 0 0.5] Enemy
  (if (< (Math|Vector|VectorLengthSquared _returnvalue_8) (.predatorrangesqr _boidinfo))
    (Variables|Default|SetPredatorDir (Math|Vector|Normalize _returnvalue_8))
    (else
      (Variables|Default|SetPredatorDir "0, 0, 0")))
  ;[0.15 0.15 0.15 0.5] Combine
  (Variables|Default|SetDirection (Math|Vector|Normalize (Math|Vector|Lerp(Vector) (Variables|Default|GetDirection) (Math|Vector|Normalize (Math|Vector|MakeVector (.x (+ (+ (+ (+ (* (Math|Vector|Normalize (Variables|Default|GetCohesionDir)) (.cohesionstrength _boidinfo_2)) (* (Math|Vector|Normalize (Variables|Default|GetAlignmentDir)) (.alignmentstrength _boidinfo_2))) (* (Math|Vector|Normalize (Variables|Default|GetSeparationDir)) (.separationstrength _boidinfo_2))) (* (Math|Random|RandomUnitVector) (.randomstrength _boidinfo_2))) (* (Variables|Default|GetPredatorDir) (.predatorstrength _boidinfo_2)))) (.y (+ (+ (+ (+ (* (Math|Vector|Normalize (Variables|Default|GetCohesionDir)) (.cohesionstrength _boidinfo_2)) (* (Math|Vector|Normalize (Variables|Default|GetAlignmentDir)) (.alignmentstrength _boidinfo_2))) (* (Math|Vector|Normalize (Variables|Default|GetSeparationDir)) (.separationstrength _boidinfo_2))) (* (Math|Random|RandomUnitVector) (.randomstrength _boidinfo_2))) (* (Variables|Default|GetPredatorDir) (.predatorstrength _boidinfo_2)))) 0.0)) (* (Variables|Default|GetRotateSpeed) (Variables|Default|GetUpdateRate))))))

(event Custom|Anim%20Beeds
  (bind _wingr (Variables|Default|GetWingR))
  (bind _wingl (Variables|Default|GetWingL))
  (bind (_direction _alpha_rota _alpha_scale) (Timeline|Anim PlayFromStart)
    (:Update
      (Transformation|SetRelativeRotation _wingl (Math|Rotator|Lerp(Rotator) "-10.000000,0.000000,0.000000" "40.000000,0.000000,0.000000" _alpha_rota) false false)
      (Transformation|SetRelativeScale3D _wingl (Math|Vector|Lerp(Vector) "-0.800000,1.200000,1.000000" "-1.200000,0.800000,1.000000" _alpha_scale))
      (Transformation|SetRelativeRotation _wingr (Math|Rotator|Lerp(Rotator) "10.000000,0.000000,0.000000" "-40.000000,0.000000,0.000000" _alpha_rota) false false)
      (Transformation|SetRelativeScale3D _wingr (Math|Vector|Lerp(Vector) "0.800000,1.200000,1.000000" "1.200000,0.800000,1.000000" _alpha_scale)))
    (:Finished
      (CallFunction|AnimBeeds))))

(event Custom|OnComponentBeginOverlap_Event
  (params (OverlappedComponent :type Primitive%20Component%20Object%20Reference) (OtherActor :type Actor%20Object%20Reference) (OtherComp :type Primitive%20Component%20Object%20Reference) (OtherBodyIndex :type Integer) (bFromSweep :type Boolean) (SweepResult :type Hit%20Result%20Structure%20%28by%20ref%29))
  (if (Variables|Default|GetInitialized)
    (switch int (Variables|Default|GetTeam)
      (:0
        (bind _asbp_player_two (Utilities|Casting|CastToBP_PlayerTwo OtherActor))
        (Class|BPIInteract|MakeDamage(Message) (Actor|GetComponentbyClass _asbp_player_two "/Game/Blueprint/Masks/AC_MaskManager.AC_MaskManager_C") 1e+01))
      (:1
        (bind _asbp_player_one (Utilities|Casting|CastToBP_PlayerOne OtherActor))
        (Class|BPIInteract|MakeDamage(Message) (Actor|GetComponentbyClass _asbp_player_one "/Game/Blueprint/Masks/AC_MaskManager.AC_MaskManager_C") 1e+01)))
    (Actor|DestroyActor)))

(event EventBeginPlay
  (Utilities|Time|SetTimerbyEvent (delegate Custom|Update) (Variables|Default|GetUpdateRate) true true)
  (CallFunction|AnimBeeds)
  (Collision|AssignOnComponentBeginOverlap (Variables|Default|GetSphere) (delegate Custom|OnComponentBeginOverlap_Event)))

(event EventTick
  (params (DeltaSeconds :type Float%20%28single-precision%29))
  (bind _direction (Variables|Default|GetDirection))
  (CallFunction|AvoidWalls)
  (Transformation|SetActorLocationAndRotation (+ (* DeltaSeconds (* _direction (Variables|Default|GetSpeed))) (Transformation|GetActorLocation)) (Math|Rotator|CombineRotators (Math|Rotator|MakeRotfromX _direction) "0.000000,-90.000000,0.000000")))

(fn ConstructionScript)

(fn AvoidWalls
  (bind _returnvalue (Transformation|GetActorLocation))
  (bind _returnvalue_2 (Transformation|GetActorLocation))
  (bind _boidinfo (Variables|Default|GetBoidInfo))
  (bind _toignore (LocalVariables|GetToIgnore))
  (bind _toignore_2 (LocalVariables|GetToIgnore))
  (Utilities|Array|Clear _toignore)
  (bind _outactors (Actor|GetAllActorsOfClass "BP_Beeds_C"))
  (Utilities|Array|AppendArray _toignore _outactors)
  (bind _outactors_2 (Actor|GetAllActorsOfClass "/Game/Blueprint/Players/BP_PlayerParent.BP_PlayerParent_C"))
  (Utilities|Array|AppendArray _toignore _outactors_2)
  (bind _outhit (Collision|LineTraceByChannel _returnvalue_2 (+ _returnvalue_2 (* (Math|Vector|RotateVectorAroundAxis (Variables|Default|GetDirection) -15.0 "0.000000,0.000000,1.000000") (LocalVariables|GetDistance))) "TraceTypeQuery1" false _toignore_2 "None"))
  (bind _outhit_2 (Collision|LineTraceByChannel _returnvalue (+ _returnvalue (* (Math|Vector|RotateVectorAroundAxis (Variables|Default|GetDirection) 15.0 "0.000000,0.000000,1.000000") (LocalVariables|GetDistance))) "TraceTypeQuery1" false _toignore_2 "None"))
  (if (or (.bblockinghit _outhit) (.bblockinghit _outhit_2))
    (if (< (.distance _outhit) (.distance _outhit_2))
      (Variables|Default|SetDirection (Math|Vector|RotateVectorAroundAxis (Variables|Default|GetDirection) (.avoidwallstrength _boidinfo) "0.000000,0.000000,1.000000"))
      (else
        (Variables|Default|SetDirection (Math|Vector|RotateVectorAroundAxis (Variables|Default|GetDirection) (.avoidwallstrength _boidinfo) "0.000000,0.000000,1.000000"))))))

(fn Initialize
  (params (Team :type Integer) (Direction :type Vector))
  (Variables|Default|SetInitialized true)
  (Variables|Default|SetDirection Direction)
  (bind _output_get (Variables|Default|SetTeam Team))
  (switch int _output_get
    (:0
      (Components|StaticMesh|SetStaticMesh (Variables|Default|GetStaticMesh) "/Game/Assets/SM_Beed_00.SM_Beed_00"))
    (:1
      (Components|StaticMesh|SetStaticMesh (Variables|Default|GetStaticMesh) "/Game/Assets/SM_Beed2_00.SM_Beed2_00"))))