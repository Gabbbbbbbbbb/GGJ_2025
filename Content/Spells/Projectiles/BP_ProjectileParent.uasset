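; Base spell projectile that deals damage on contact and then destroys itself.
; Its sphere overlap ignores the player character identified by Launcher and sends Damage to any other actor through that actor's AC_MaskManager component.
; Before destruction it detaches the particle and ribbon effects, so they are left behind at the impact point.
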(event OnComponentBeginOverlap(Sphere)
  (params (OverlappedComponent :type Primitive%20Component%20Object%20Reference) (OtherActor :type Actor%20Object%20Reference) (OtherComp :type Primitive%20Component%20Object%20Reference) (OtherBodyIndex :type Integer) (bFromSweep :type Boolean) (SweepResult :type Hit%20Result%20Structure%20%28by%20ref%29))
  (if (!= OtherActor (Game|GetPlayerCharacter (Variables|Default|GetLauncher)))
    (Class|BPIInteract|MakeDamage(Message) (Actor|GetComponentbyClass OtherActor "/Game/Blueprint/Masks/AC_MaskManager.AC_MaskManager_C") (Variables|Default|GetDamage))
    (Transformation|DetachFromComponent (Variables|Default|GetNS_Particles) "KeepRelative" "KeepRelative" "KeepRelative" true)
    (Actor|DestroyActor)))

(event EventBeginPlay)

(fn ConstructionScript)