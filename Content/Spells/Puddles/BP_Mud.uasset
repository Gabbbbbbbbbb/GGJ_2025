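; BP_Mud is a spell puddle that slows the opposing player in a two-player setup for a limited time.
; On BeginPlay it passes Lifetime to its Niagara effect, then destroys itself when that time elapses.
; Sphere overlaps by any actor other than the Launcher's character lower the other player's walk speed.
; End overlap sets a hardcoded normal speed rather than restoring the previous value.
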(event OnComponentBeginOverlap(Sphere)
  (params (OverlappedComponent :type Primitive%20Component%20Object%20Reference) (OtherActor :type Actor%20Object%20Reference) (OtherComp :type Primitive%20Component%20Object%20Reference) (OtherBodyIndex :type Integer) (bFromSweep :type Boolean) (SweepResult :type Hit%20Result%20Structure%20%28by%20ref%29))
  (if (!= OtherActor (Game|GetPlayerCharacter (Variables|Default|GetLauncher)))
    (if (== (Variables|Default|GetLauncher) 0)
      (Variables|/Script/Engine.CharacterMovementComponent|SetMaxWalkSpeed (Variables|/Script/Engine.Character|GetCharacterMovement (Game|GetPlayerCharacter 1)) 2e+02)
      (else
        (Variables|/Script/Engine.CharacterMovementComponent|SetMaxWalkSpeed (Variables|/Script/Engine.Character|GetCharacterMovement (Game|GetPlayerCharacter 0)) 2e+02)))))

(event OnComponentEndOverlap(Sphere)
  (params (OverlappedComponent :type Primitive%20Component%20Object%20Reference) (OtherActor :type Actor%20Object%20Reference) (OtherComp :type Primitive%20Component%20Object%20Reference) (OtherBodyIndex :type Integer))
  (if (!= OtherActor (Game|GetPlayerCharacter (Variables|Default|GetLauncher)))
    (if (== (Variables|Default|GetLauncher) 0)
      (Variables|/Script/Engine.CharacterMovementComponent|SetMaxWalkSpeed (Variables|/Script/Engine.Character|GetCharacterMovement (Game|GetPlayerCharacter 1)) 6e+02)
      (else
        (Variables|/Script/Engine.CharacterMovementComponent|SetMaxWalkSpeed (Variables|/Script/Engine.Character|GetCharacterMovement (Game|GetPlayerCharacter 0)) 6e+02)))))

(event EventBeginPlay
  (bind _lifetime (Variables|Default|GetLifetime))
  (Effects|Components|ParticleSystem|SetFloatParameter (Variables|Default|GetNS_Puddle) "Lifetime" _lifetime)
  (Utilities|FlowControl|Delay _lifetime)
  (Actor|DestroyActor))

(fn ConstructionScript
  (|CallParentFunction))