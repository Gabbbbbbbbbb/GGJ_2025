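; Poison puddle spell actor that damages characters standing in it, excluding the player character of its launcher.
; On BeginPlay it passes its lifetime to the Niagara puddle effect, then destroys itself after that delay.
; Sphere overlap starts a delay loop that repeatedly sends damage through the target's AC_MaskManager component.
; One shared in-zone flag, set on overlap begin and cleared on end, gates the loop for all targets.
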(event OnComponentBeginOverlap(Sphere)
  (params (OverlappedComponent :type Primitive%20Component%20Object%20Reference) (OtherActor :type Actor%20Object%20Reference) (OtherComp :type Primitive%20Component%20Object%20Reference) (OtherBodyIndex :type Integer) (bFromSweep :type Boolean) (SweepResult :type Hit%20Result%20Structure%20%28by%20ref%29))
  (if (!= OtherActor (Game|GetPlayerCharacter (Variables|Default|GetLauncher)))
    (Variables|Default|SetIsInZone true)
    (Variables|Default|GetIsInZone :!label _label
      (:then
        (Class|BPIInteract|MakeDamage(Message) (Actor|GetComponentbyClass OtherActor "/Game/Blueprint/Masks/AC_MaskManager.AC_MaskManager_C") (Variables|Default|GetDamages))
        (Utilities|FlowControl|Delay (Variables|Default|GetTimeBeforeEffect))
        (goto _label))
      (:else))))

(event OnComponentEndOverlap(Sphere)
  (params (OverlappedComponent :type Primitive%20Component%20Object%20Reference) (OtherActor :type Actor%20Object%20Reference) (OtherComp :type Primitive%20Component%20Object%20Reference) (OtherBodyIndex :type Integer))
  (if (!= OtherActor (Game|GetPlayerCharacter (Variables|Default|GetLauncher)))
    (Variables|Default|SetIsInZone false)))

(event EventBeginPlay
  (bind _lifetime (Variables|Default|GetLifetime))
  (Effects|Components|ParticleSystem|SetFloatParameter (Variables|Default|GetNS_Puddle) "Lifetime" _lifetime)
  (Utilities|FlowControl|Delay _lifetime)
  (Actor|DestroyActor))

(fn ConstructionScript
  (|CallParentFunction))