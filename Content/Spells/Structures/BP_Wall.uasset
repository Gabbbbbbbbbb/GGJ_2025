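; BP_Wall is a temporary wall structure, filed under spell structures, that rises out of the ground when spawned.
; A Spawn timeline lerps the cube's relative location up from below, then after a Duration delay a second timeline sinks it back and destroys the actor.
; A Remove event plays that sinking timeline directly, allowing the wall to be dismissed early.
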(event Custom|Remove
  (bind _spawn (Timeline|Timeline PlayFromStart)
    (:Update
      (Transformation|SetRelativeLocation (Variables|Default|GetCube) (Math|Vector|Lerp(Vector) "0, 0, 0" "0.000000,0.000000,-100.000000" _spawn) false false))
    (:Finished
      (Actor|DestroyActor))))

(event EventBeginPlay
  (bind _spawn (Timeline|Spawn PlayFromStart)
    (:Update
      (Transformation|SetRelativeLocation (Variables|Default|GetCube) (Math|Vector|Lerp(Vector) "0.000000,0.000000,-100.000000" "0, 0, 0" _spawn) false false))
    (:Finished
      (Utilities|FlowControl|Delay (Variables|Default|GetDuration))
      (bind _spawn_2 (Timeline|Timeline PlayFromStart)
        (:Update
          (Transformation|SetRelativeLocation (Variables|Default|GetCube) (Math|Vector|Lerp(Vector) "0, 0, 0" "0.000000,0.000000,-100.000000" _spawn_2) false false))
        (:Finished
          (Actor|DestroyActor))))))

(fn ConstructionScript)